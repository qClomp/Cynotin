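; Player controller for the character creation menu, which shows the menu widget and switches input to UI only on BeginPlay.
; A CreateWidget helper creates the widget, adds it to the viewport and sets its visibility.
; E_MouseLineTrace, which is not called within this Blueprint, starts a looping timer that line traces from the deprojected mouse position, with persistent debug drawing and printed hit results.
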(event Custom|E_MouseLineTrace
  (Utilities|Time|SetTimerbyEvent (delegate Custom|E_LineTrace) 0.2 true))

(event Custom|E_LineTrace
  (bind _self self)
  (bind (_worldlocation _worlddirection) (Game|Player|ConvertMouseLocationToWorldSpace _self))
  (bind (_outhit _returnvalue) (Collision|LineTraceByChannel (- _worldlocation (Math|Float|MakeLiteralFloat 1e+01)) (* (+ (Math|Vector|GetForwardVector (Pawn|GetControlRotation _self :!class /Script/Engine.Controller)) (Math|Float|MakeLiteralFloat 1e+03)) _worlddirection) "TraceTypeQuery3" false 0 "Persistent"))
  (Development|PrintString (Utilities|String|ToString(Boolean) _returnvalue))
  (Development|PrintString (Utilities|GetDisplayName (.HitActor (Collision|BreakHitResult _outhit)))))

(event EventBeginPlay
  (Input|SetInputModeUIOnly self 0 "DoNotLock")
  (Utilities|CreateWidget "/Game/UserInterface/CharacterCreationMenu/UI_CharacterCreationMenu.UI_CharacterCreationMenu_C" "Visible"))

(event EventTick
  (params (DeltaSeconds :type Float%20%28single-precision%29)))

(fn ConstructionScript)
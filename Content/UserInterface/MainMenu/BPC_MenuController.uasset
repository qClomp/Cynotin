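; Player controller for the main menu that manages switching between the main menu and character selection screens.
; On BeginPlay it creates both widgets up front through a CreateWidget helper, with character selection hidden, and sets UI-only input.
; Screen-switch events fire LevelToCharacterSelection or LevelToMainMenu, hide the passed-in widget and show the target.
; A separate event opens the character creation level.
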(event Custom|Init%20Widgets
  ;[1 1 1] Comment
  (bind _outputpin (Utilities|CreateWidget "/Game/UserInterface/MainMenu/UI_MainMenu.UI_MainMenu_C" "Visible"))
  (Variables|Default|SetUI_MainMenu _outputpin)
  (bind _outputpin_2 (Utilities|CreateWidget "/Game/UserInterface/MainMenu/CharacterSelectionMenu/UI_CharacterSelection.UI_CharacterSelection_C" "Hidden"))
  (Variables|Default|SetUI_CharacterSelection _outputpin_2))

(event EventBeginPlay
  (CallFunction|InitWidgets)
  (Input|SetInputModeUIOnly self 0 "DoNotLock"))

(event EventTick
  (params (DeltaSeconds :type Float%20%28single-precision%29)))

(event EventToCharacterSelectionScreen
  (params (ReferenceSelf :type User%20Widget%20Object%20Reference))
  (Default|CallLeveltoCharacterSelection)
  (Widget|SetVisibility ReferenceSelf "Hidden")
  (Widget|SetVisibility (Variables|Default|GetUI_CharacterSelection) "Visible"))

(event EventToMainMenu
  (params (ReferenceSelf :type User%20Widget%20Object%20Reference))
  (Default|CallLeveltoMainMenu)
  (Widget|SetVisibility ReferenceSelf "Hidden")
  (Widget|SetVisibility (Variables|Default|GetUI_MainMenu) "Visible"))

(event EventToCharacterCreationMenu
  (params (ReferenceSelf :type User%20Widget%20Object%20Reference))
  (Game|OpenLevel(byName) "L_CharacterCreationLevel"))

(fn ConstructionScript)
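; Loot box actor that holds one item class and lets the player collect it into their inventory with the E button.
; SetItemInsideBox stores the class and builds the widget showing it; BeginPlay fills in a placeholder weapon, marked for deletion.
; Box overlap by a PlayerCharacter-tagged actor enables interaction and shows the widget.
; E, bound through a controller interface, adds the item via the HUD's inventory interface and destroys the box on success.
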(event OnComponentBeginOverlap(Box)
  (params (OverlappedComponent :type Primitive%20Component%20Object%20Reference) (OtherActor :type Actor%20Object%20Reference) (OtherComp :type Primitive%20Component%20Object%20Reference) (OtherBodyIndex :type Integer) (bFromSweep :type Boolean) (SweepResult :type Hit%20Result%20Structure%20%28by%20ref%29))
  ;[1 1 1] Comment
  (if (Actor|ActorHasTag OtherActor "PlayerCharacter")
    (Variables|Default|SetCanInteract true)
    (Rendering|SetVisibility (Variables|Default|GetWidget) true true)))

(event OnComponentEndOverlap(Box)
  (params (OverlappedComponent :type Primitive%20Component%20Object%20Reference) (OtherActor :type Actor%20Object%20Reference) (OtherComp :type Primitive%20Component%20Object%20Reference) (OtherBodyIndex :type Integer))
  ;[1 1 1] Comment
  (Variables|Default|SetCanInteract false)
  (Rendering|SetVisibility (Variables|Default|GetWidget) false false))

(event Custom|E_Interaction_Button_E
  (if (Utilities|IsValidClass (Variables|Default|GetItemActorClass))
    (if (Variables|Default|GetCanInteract)
      (bind _inventoryreference (Class|BPIHUD|GetInventoryReference(Message) (HUD|GetHUD (Game|GetPlayerController 0))))
      (bind _succes (Class|BPIInventory|InventoryAddItem(Message) _inventoryreference (Variables|Default|GetItemActorClass)))
      (if _succes
        (Actor|DestroyActor)))))

(event EventBeginPlay
  ;[1 1 1] Delete
  (CallFunction|SetItemInsideBox "/Game/Assets/Weapons/ph_weapon/Weapon_ph_weapon.Weapon_ph_weapon_C")
  (bind _bpc_charactercontroller (Class|BPICharacterController|GetReferencePlayerController(Message) (Game|GetPlayerController 0)))
  (EventDispatchers|BindEventtoButtonE _bpc_charactercontroller (delegate Custom|E_Interaction_Button_E)))

(event Collision|EventActorBeginOverlap
  (params (OtherActor :type Actor%20Object%20Reference)))

(event EventTick
  (params (DeltaSeconds :type Float%20%28single-precision%29)))

(event EventSetItemInsideBox
  (params (ActorClasses :type Actor%20Class%20Reference))
  (bind _output_get (Variables|Default|SetItemActorClass ActorClasses))
  (bind _returnvalue (UserInterface|CreateWidget "/Game/Assets/Loot/UI_LootBox.UI_LootBox_C"))
  (UserInterface|SetWidget (Variables|Default|GetWidget) _returnvalue)
  (Default|WidgetItem _returnvalue _output_get))

(fn ConstructionScript)
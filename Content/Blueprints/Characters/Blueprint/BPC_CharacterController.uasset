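; Player controller for BP_Character that handles movement, camera, weapons and HUD toggles for inventory and settings.
; Movement, spring-arm look with mesh turning, timeline-blended stepped zoom, and firing run only in the Main player state.
; Firing while armed auto-enters aim through the weapon system, changing walk speed, then exits aim on release via a gate.
; Every tick, a camera-forward line trace notifies the hit actor through a message.
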(event Custom|E_ReferenceCharacter
  ;[1 1 1] Reference Character
  (bind _asbp_character (Utilities|Casting|CastToBP_Character (Game|GetPlayerCharacter 0)))
  (Variables|MainReferences|SetBP_Character _asbp_character)
  (Variables|MainReferences|SetMain%20Camera (Variables|/Game/Blueprints/Characters/Blueprint/BP_Character.BP_Character_C|GetMainCamera _asbp_character))
  (Variables|MainReferences|SetSpring%20Arm (Variables|/Game/Blueprints/Characters/Blueprint/BP_Character.BP_Character_C|GetSpringArm _asbp_character))
  (Variables|MainReferences|SetCharacter%20Movement (Variables|/Script/Engine.Character|GetCharacterMovement _asbp_character)))

(event Custom|E_StartAim
  ;[0 0 0] Delete
  ;;[1 1 1] Player Aim | (Zoom)
  (bind _weaponisvalid (Default|CharacterAimWeapon (Variables|Default|GetBPA_WeaponSystem)))
  (bind _output_get (Variables|Player|SetPlayerAiming _weaponisvalid))
  (if _output_get
    (Utilities|SetCharacterWalkSpeed (Math|Float|MakeLiteralFloat 3e+02)))
  ;;;[1 1 1] Camera Zoom
  (bind _output_get_2 (Variables|Aim|SetStore_TargetArmLengthForAim 6e+02))
  (bind _lerptime (Timeline|Timeline_0 PlayFromStart)
    (:Update
      (Utilities|SetTargetArmLength (Math|Float|Lerp _output_get_2 (Math|Float|MakeLiteralFloat 6e+02) _lerptime)))))

(event Custom|E_EndAim
  ;[0 0 0] Delete
  ;;[1 1 1] Player Aim | (Zoom)
  (Default|CharacterHolsterWeapon (Variables|Default|GetBPA_WeaponSystem))
  (Variables|Player|SetPlayerAiming false)
  (Utilities|SetCharacterWalkSpeed (Math|Float|MakeLiteralFloat 2e+03))
  ;;;[1 1 1] Camera Zoom
  (bind _lerptime (Timeline|Timeline_1 PlayFromStart)
    (:Update
      (Utilities|SetTargetArmLength (Math|Float|Lerp (Math|Float|MakeLiteralFloat 6e+02) (Variables|Aim|GetStore_TargetArmLengthForAim) _lerptime))
      (Variables|Camera|SetCurrentCameraZoom 2))))

(event EventBeginPlay
  ;[1 1 1] BeginPlay
  (CallFunction|EReferenceCharacter)
  (bind _hudreference (Class|BPIHUD|GetHUDReference(Message) (HUD|GetHUD)))
  (Variables|HUD|SetPlayerHUD1 _hudreference))

(event EventSetPlayerState
  (params (PlayerState :type enum_PlayerStates%20Enum :default "NewEnumerator0"))
  ;[1 1 1] BPI_Set Player State
  (Variables|Default|SetPlayerStates PlayerState))

(event EventTick
  (params (DeltaSeconds :type Float%20%28single-precision%29))
  ;[1 1 1] Character Line Trace
  (bind (_hitresult _hit) (CallFunction|CharacterDrawLineTrace))
  (if _hit
    (Class|BPILineTrace|LineTraceHit(Message) (.HitActor (Collision|BreakHitResult _hitresult)) self)))

(event EventInitCharacterAnimation
  (params (AnimationBP :type Object%20Object%20Reference))
  ;[1 1 1] Character Animation Blueprint
  (Variables|MainReferences|SetBPA_Character AnimationBP))

(event Input|AxisEvents|InputAxisMoveForward
  (params (AxisValue :type Float%20%28single-precision%29))
  (bind _bp_character (Variables|MainReferences|GetBP_Character))
  ;[1 1 1] PlayerMovement | WASD Movement
  (Utilities|GetPlayerStates
    (:MainState
      (if (!= AxisValue 0.0)
        (Pawn|Input|AddMovementInput _bp_character (Math|Vector|GetForwardVector (Variables|/Game/Blueprints/Characters/Blueprint/BP_Character.BP_Character_C|GetDirectionArrow _bp_character)) AxisValue false)
        (CallFunction|FSetPlayerRotation AxisValue (stale Input|AxisEvents|InputAxisMoveRight AxisValue))))))

(event Input|AxisEvents|InputAxisMoveRight
  (params (AxisValue :type Float%20%28single-precision%29))
  (bind _bp_character (Variables|MainReferences|GetBP_Character))
  ;[1 1 1] PlayerMovement | WASD Movement
  (Utilities|GetPlayerStates
    (:MainState
      (if (!= AxisValue 0.0)
        (Pawn|Input|AddMovementInput _bp_character (Math|Vector|GetRightVector (Variables|/Game/Blueprints/Characters/Blueprint/BP_Character.BP_Character_C|GetDirectionArrow _bp_character)) AxisValue false)
        (CallFunction|FSetPlayerRotation (stale Input|AxisEvents|InputAxisMoveForward AxisValue) AxisValue)))))

(event Input|AxisEvents|InputAxisLookUp
  (params (AxisValue :type Float%20%28single-precision%29))
  ;[1 1 1] CameraMovement | Camera LookUp
  (Utilities|GetPlayerStates
    (:MainState
      (if (!= AxisValue 0.0)
        (if (> AxisValue 0.0)
          (if (<= (.Pitch (Math|Rotator|BreakRotator (Transformation|GetWorldRotation (Variables|MainReferences|GetSpring%20Arm)))) 3e+01)
            (Transformation|AddRelativeRotation (Variables|MainReferences|GetSpring%20Arm) (Math|Rotator|MakeRotator 0.0 AxisValue 0.0) false false :!label _label))
          (elif (< AxisValue 0.0)
            (if (>= (.Pitch (Math|Rotator|BreakRotator (Transformation|GetWorldRotation (Variables|MainReferences|GetSpring%20Arm)))) -5e+01)
              (goto _label))))))))

(event Input|AxisEvents|InputAxisLookRight
  (params (AxisValue :type Float%20%28single-precision%29))
  ;[1 1 1] CameraMovement | LookRight
  (Utilities|GetPlayerStates
    (:MainState
      (Transformation|AddWorldRotation (Variables|MainReferences|GetSpring%20Arm) (Math|Rotator|MakeRotator 0.0 0.0 AxisValue) false false)
      (Transformation|SetWorldRotation (Variables|/Script/Engine.Character|GetMesh (Variables|MainReferences|GetBP_Character)) (Math|Interpolation|RInterpTo (Math|Rotator|MakeRotator 0.0 0.0 (.Yaw (Math|Rotator|BreakRotator (Transformation|GetWorldRotation (Variables|/Script/Engine.Character|GetMesh (Variables|MainReferences|GetBP_Character)))))) (Math|Rotator|MakeRotator 0.0 0.0 (+ (.Yaw (Math|Rotator|BreakRotator (Class|SpringArmComponent|GetTargetRotation (Variables|MainReferences|GetSpring%20Arm)))) -9e+01)) (Utilities|Time|GetWorldDeltaSeconds) 4e+01) false false))))

(event Input|AxisEvents|InputAxisZoomInOut
  (params (AxisValue :type Float%20%28single-precision%29))
  ;[1 1 1] CameraMovement | Zoom
  (Utilities|GetPlayerStates
    (:MainState
      (Utilities|BiggerBranch (!= AxisValue 0.0) (not (Variables|Player|GetPlayerAiming)) true true true true true
        (:true
          (bind (_valid_ _currentarmlength _targetarmlength _updatedzoomlevel) (CallFunction|FCameraZoom AxisValue))
          (if _valid_
            (Variables|Camera|SetCurrentCameraZoom _updatedzoomlevel)
            (bind _zoomtime (Timeline|CameraZoomInOut PlayFromStart)
              (:Update
                (Utilities|SetTargetArmLength (Math|Float|Lerp _currentarmlength _targetarmlength _zoomtime))))))))))

(event Input|MouseEvents|RightMouseButton
  (params (Key :type Key%20Structure :default "None"))
  ;[0 0 0] Delete
  ;;[1 1 1] Player Aim | RightClick
)

(event Input|KeyboardEvents|Escape
  (params (Key :type Key%20Structure :default "None"))
  ;[1 1 1] Comment
  (:Pressed
    (Utilities|FlowControl|FlipFlop
      (:A
        (Class|BPIHUD|InGameSettingsOpen(Message) (Utilities|GetMHUD)))
      (:B
        (Class|BPIHUD|InGameSettingsClose(Message) (Utilities|GetMHUD))))))

(event Input|KeyboardEvents|5
  (params (Key :type Key%20Structure :default "None"))
  (:Pressed
    (Utilities|FlowControl|FlipFlop
      (:A
        (Variables|Default|SetbShowMouseCursor true))
      (:B
        (Variables|Default|SetbShowMouseCursor false)))))

(event Input|KeyboardEvents|Tab
  (params (Key :type Key%20Structure :default "None"))
  ;[1 1 1] Inventory
)

(event Input|KeyboardEvents|T
  (params (Key :type Key%20Structure :default "None"))
  ;[1 1 1] Test
  (:Pressed
    (bind _inventoryreference (Utilities|GetInventoryWidget))
    (Class|BPIInventory|InventoryAddItem(Message) _inventoryreference "/Game/Assets/Weapons/ph_weapon/Weapon_ph_weapon.Weapon_ph_weapon_C")))

(event Input|KeyboardEvents|Q
  (params (Key :type Key%20Structure :default "None"))
  (bind _playerhud1 (Utilities|GetMHUD))
  ;[1 1 1] Inventory
  (:Pressed
    (Utilities|FlowControl|FlipFlop
      (:A
        (Class|BPIHUD|InventoryOpen(Message) _playerhud1))
      (:B
        (Class|BPIHUD|InventoryClose(Message) _playerhud1)))))

(event Input|KeyboardEvents|Z
  (params (Key :type Key%20Structure :default "None"))
  ;[1 1 1] Z X V | Equip Weapon
  (:Pressed
    (if (not (Variables|Player|GetPlayerAiming))
      (bind _zisvalid (Default|WeaponSetZActive (Variables|Default|GetBPA_WeaponSystem)))
      (if _zisvalid
        (Variables|Default|SetPlayerArmed true)
        (else
          (Variables|Default|SetPlayerArmed false))))))

(event Input|KeyboardEvents|X
  (params (Key :type Key%20Structure :default "None"))
  ;[1 1 1] Z X V | Equip Weapon
)

(event Input|MouseEvents|LeftMouseButton
  (params (Key :type Key%20Structure :default "None"))
  ;[1 1 1] Shoot | Left Mouse Button
  (:Pressed
    (Utilities|GetPlayerStates
      (:MainState
        (if (Variables|Player|GetPlayerAiming)
          (Class|BPIWeaponSystem|WeaponStartShooting(Message) (Variables|Default|GetBPA_WeaponSystem))
          (elif (Variables|Default|GetPlayerArmed)
            (Utilities|FlowControl|Sequence
              (:then_0
                (CallFunction|EStartAim)
                (Class|BPIWeaponSystem|WeaponStartShooting(Message) (Variables|Default|GetBPA_WeaponSystem)))
              (:then_1
                (goto _label Open))))))))
  (:Released
    (Class|BPIWeaponSystem|WeaponStopShooting(Message) (Variables|Default|GetBPA_WeaponSystem))
    (Utilities|FlowControl|Gate true :!label _label
      (:Exit
        (CallFunction|EEndAim)
        (goto _label Close)))))

(event Input|KeyboardEvents|E
  (params (Key :type Key%20Structure :default "None"))
  (:Pressed
    (Default|CallButtonE)))

(fn ConstructionScript)

(fn FSetPlayerRotation
  (params (ForwardScalarValue :type Float%20%28single-precision%29) (RightScalarValue :type Float%20%28single-precision%29))
  (Utilities|FlowControl|Sequence
    (:then_0
      ;[1 1 1] W
      (if (> ForwardScalarValue 0.0)
        (LocalVariables|SetForwardX 0.0)
        (if true :!label _label
          (Variables|Player|SetPlayerRotationForwardWS (LocalVariables|GetForwardX))
          (Variables|Player|SetPlayerRotationRightAD (LocalVariables|GetRightY)))
        (else
          ;[1 1 1] S
          (if (> 0.0 ForwardScalarValue)
            (LocalVariables|SetForwardX 1.8e+02)
            (goto _label)))))
    (:then_1
      ;[1 1 1] D
      (if (> RightScalarValue 0.0)
        (LocalVariables|SetRightY 9e+01)
        (goto _label)
        (else
          ;[1 1 1] A
          (if (> 0.0 RightScalarValue)
            (LocalVariables|SetRightY -9e+01)
            (goto _label)))))))

(fn FCameraZoom
  (params (AxisValue :type Float%20%28single-precision%29))
  (bind _currentcamerazoom (Variables|Camera|GetCurrentCameraZoom))
  (bind _currentcamerazoom_2 (Variables|Camera|GetCurrentCameraZoom))
  (bind _returnvalue (- _currentcamerazoom_2 1))
  (bind _returnvalue_2 (+ _currentcamerazoom 1))
  (LocalVariables|SetCurrentCameraArmLength (Utilities|GetTargetArmLength))
  (if (> AxisValue 0.0)
    (return (> _returnvalue 0) (LocalVariables|GetCurrentCameraArmLength) (.Value (Utilities|Map|Find (Variables|Camera|GetCameraZoomLevels) _returnvalue)) _returnvalue)
    (elif (< AxisValue 0.0)
      (return (< _returnvalue_2 5) (LocalVariables|GetCurrentCameraArmLength) (.Value (Utilities|Map|Find (Variables|Camera|GetCameraZoomLevels) _returnvalue_2)) _returnvalue_2))))

(fn FAimWalkArmed
  (params (SetActive :type Boolean) (DeActive :type Boolean))
  (if SetActive
    (Variables|Player|SetPlayerAiming true)
    (Variables|/Script/Engine.CharacterMovementComponent|SetMaxWalkSpeed (Variables|MainReferences|GetCharacter%20Movement) 3e+02)
    (Variables|Aim|SetStore_TargetArmLengthForAim (Variables|/Script/Engine.SpringArmComponent|GetTargetArmLength (Variables|MainReferences|GetSpring%20Arm)))
    (Variables|/Script/Engine.SpringArmComponent|SetTargetArmLength (Variables|MainReferences|GetSpring%20Arm) 3e+02)
    (elif DeActive
      (Variables|Player|SetPlayerAiming false)
      (Variables|/Script/Engine.CharacterMovementComponent|SetMaxWalkSpeed (Variables|MainReferences|GetCharacter%20Movement) 6e+02)
      (Variables|/Script/Engine.SpringArmComponent|SetTargetArmLength (Variables|MainReferences|GetSpring%20Arm) (Variables|Aim|GetStore_TargetArmLengthForAim)))))

(fn ItemSlotEmpty
  (return false))

(fn InventoryAddItem
  (params (itemstructure :type Structure%20Item%20Structure))
  (return false))

(fn GetWeaponStructure
  (return ""))

(fn GetPlayerInterfaceReference
  (return 0))

(fn GetInventoryReference)

(fn InventoryOpen)

(fn GetHUDReference
  (return 0))

(fn CharacterAnimationBP
  (return (Variables|MainReferences|GetBPA_Character)))

(fn CharacterDrawLineTrace
  (bind _main_camera (Variables|MainReferences|GetMain%20Camera))
  (bind _returnvalue (Transformation|GetWorldLocation _main_camera))
  (bind (_outhit _returnvalue_2) (Collision|LineTraceByChannel _returnvalue (+ _returnvalue (* (Math|Vector|GetForwardVector (Transformation|GetWorldRotation _main_camera)) (Math|Float|MakeLiteralFloat 1e+04))) "TraceTypeQuery3" false 0 "None"))
  (return _outhit _returnvalue_2))

(fn CharacterGetLocation
  (return (Transformation|GetWorldLocation (Variables|/Script/Engine.Character|GetMesh (Variables|MainReferences|GetBP_Character)))))

(fn GetReferencePlayerController
  (return self))